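; AI enemy character that idles, roams, fights and flees from the player, driven by a boolean state machine on Tick rather than a Behavior Tree.
; Line-trace vision with a range limit triggers combat, low-health retreat or pursuit to the last seen location.
; Combat alternates stepping toward the player with firing its attached weapon, spawning bullet, flash and traced explosion via interlocked DoOnce gates.
; DamageActor handles health and explosive death.
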(event EventBeginPlay
  (bind _mesh (Variables|Character|GetMesh))
  ;[1 1 1] Begin Play
  (Utilities|FlowControl|Sequence
    (:then_0
      (bind _returnvalue (Game|SpawnActorfromClass "/Game/Assets/Weapons/Guns/BendellWeapon.BendellWeapon_C" (Transformation|GetWorldTransform _mesh) "Undefined" 0 0))
      (bind _output_get (Variables|Default|SetAIWeapon _returnvalue))
      (Transformation|AttachComponentToComponent _output_get _mesh "AIWeapon" "SnapToTarget" "SnapToTarget" "KeepRelative" true))
    (:then_1
      (Variables|Default|SetTzero (Utilities|Time|GetGameTimeinSeconds)))
    (:then_2
      (Variables|Default|SetTIdleStart (Utilities|Time|GetGameTimeinSeconds))
      (Variables|Default|SetIdleState true)
      (Variables|Default|SetCurrentHealth (Variables|Default|GetHealth))
      (Variables|Default|SetEnemy (Game|GetPlayerCharacter 0))
      (Variables|Default|SetAIReference self)
      (Variables|Default|SetAISpeed 4e+02))))

(event EventDamageActor
  (params (DamageAmount :type Float%20%28single-precision%29))
  ;[1 1 1] Health and Death
  (if (<= (- (Variables|Default|GetCurrentHealth) DamageAmount) 0.0)
    (Variables|Default|SetIsDead true)
    (bind _returnvalue (Game|SpawnActorfromClass "/Game/Assets/Weapons/Guns/DeathExplosion.DeathExplosion_C" (Transformation|GetWorldTransform (Variables|Default|GetSphere)) "Undefined" (Variables|Default|GetAIReference) 0))
    (Actor|DestroyActor)
    (Actor|DestroyActor (Variables|Default|GetAIWeapon))
    (Utilities|FlowControl|Delay 3.0)
    (bind _output_get (Variables|Default|SetDeathExplosion _returnvalue))
    (Actor|DestroyActor _output_get)
    (else
      (bind _output_get_2 (Variables|Default|SetCurrentHealth (- (Variables|Default|GetCurrentHealth) DamageAmount))))))

(event EventTick
  (params (DeltaSeconds :type Float%20%28single-precision%29))
  (bind _mesh (Variables|Character|GetMesh))
  (bind _aiweapon (Variables|Default|GetAIWeapon))
  (bind _aiweapon_2 (Variables|Default|GetAIWeapon))
  (bind _returnvalue (Math|Vector|GetForwardVector _mesh))
  (bind _bulletspawn (Variables|/Game/Assets/Weapons/Guns/BendellWeapon.BendellWeapon_C|GetBulletSpawn _aiweapon))
  (bind _bulletspawn_2 (Variables|/Game/Assets/Weapons/Guns/BendellWeapon.BendellWeapon_C|GetBulletSpawn _aiweapon_2))
  (bind _returnvalue_2 (Transformation|GetWorldTransform _bulletspawn_2))
  (bind _returnvalue_3 (Transformation|GetWorldLocation _bulletspawn))
  ;[1 1 1] Tick
  ;[1 1 1] IdleState
  (if (Variables|Default|GetIdleState) ; Just chilling bro?
    (Variables|/Script/Engine.CharacterMovementComponent|SetMaxWalkSpeed (Variables|/Script/Engine.Character|GetCharacterMovement (Variables|Default|GetAIReference)) (* (/ (Variables|Default|GetAISpeed) 3.0) 1.0))
    (if (Variables|Default|GetEnemyIsVisible) ; Bogies?
      (if (<= (Variables|Default|GetCurrentHealth) 2e+01) ; Ya fucked man?
        ;[1 1 1] FleeState
        (AI|AIMoveTo self (Class|NavigationSystem|GetRandomPointinNavigableRadius (- (Math|Vector|MakeVector (* (.x _returnvalue) -1e+02) (* (.y _returnvalue) -1e+02) (.z _returnvalue)) (Transformation|GetWorldLocation _mesh)) 4e+02) 0 5.0 false :!label _label ; GTFO
          (:then
            (Variables|Default|SetIsMoving true)
            (Variables|Default|SetFleeState true)
            (Variables|Default|SetCombatState false)
            (Variables|Default|SetIdleState false))
          (:OnSuccess
            (Variables|Default|SetIsMoving false :!label _label_2)
            (Variables|Default|SetFleeState false)
            (Variables|Default|SetCombatState false)
            (Variables|Default|SetIdleState true)
            (Variables|Default|SetTIdleStart (Utilities|Time|GetGameTimeinSeconds)))
          (:OnFail
            (goto _label_2)))
        (else
          ;[1 1 1] CombatState
          (Variables|Default|SetCombatState true)
          (Variables|Default|SetIdleState false)
          (Variables|Default|SetFleeState false)
          (Variables|Default|SetRoamState false)
          (Utilities|FlowControl|Sequence :!label _label_3 ; Double check enemy visible, approach enemy, fire at enemy
            (:then_0
              (bind (_targetisvisible _targetlocation) (CallFunction|AIVisionCheck (Variables|Default|GetAIReference) (Variables|Default|GetEnemy)))
              (bind _output_get (Variables|Default|SetEnemyIsVisible _targetisvisible))
              (if _output_get
                (Variables|Default|SetEnemyLocation _targetlocation)))
            (:then_1
              (if (Variables|Default|GetEnemyIsVisible)
                (if (<= (Variables|Default|GetCurrentHealth) 2e+01)
                  (goto _label)
                  (elif (not (Variables|Default|GetIsMoving))
                    ;[1 1 1] Approach
                    (Utilities|FlowControl|DoOnce false :!label _label_4
                      (:Completed
                        (bind _aitotargetrotator (CallFunction|AIAim (Variables|Default|GetEnemy)))
                        (Transformation|SetActorRotation _aitotargetrotator)
                        (bind _stepdestination (CallFunction|AIStepTowards (Variables|Default|GetEnemy)))
                        (AI|AIMoveTo self _stepdestination 0 5.0 false
                          (:then
                            (Variables|Default|SetIsMoving true))
                          (:OnSuccess
                            (Variables|Default|SetIsMoving false :!label _label_5)
                            (goto _label_7 Reset))
                          (:OnFail
                            (goto _label_5)))))))
                (else
                  (Variables|Default|SetCombatState false)
                  (Variables|Default|SetIdleState true)
                  (Variables|Default|SetFleeState false)
                  (Variables|Default|SetRoamState false)
                  ;[1 1 1] Hunt them down
                  (Development|PrintString "Hunting")
                  (AI|AIMoveTo self (Variables|Default|GetEnemyLocation) 0 5.0 false
                    (:then
                      (Variables|Default|SetIsMoving true))
                    (:OnSuccess
                      (Variables|Default|SetIsMoving false :!label _label_6)
                      (Variables|Default|SetTIdleStart (Utilities|Time|GetGameTimeinSeconds)))
                    (:OnFail
                      (goto _label_6))))))
            (:then_2
              (if (not (Variables|Default|GetIsMoving))
                (if (not (Variables|Default|GetIsFiring))
                  ;[1 1 1] Aim and Shoot
                  (Utilities|FlowControl|DoOnce false :!label _label_7
                    (:Completed
                      (Variables|Default|SetIsFiring true)
                      (Game|SpawnActorfromClass "/Game/Assets/Weapons/Guns/BendellBullet.BendellBullet_C" _returnvalue_2 "Undefined" 0 0)
                      (Game|SpawnActorfromClass "/Game/Assets/Weapons/Guns/BarrelFlash.BarrelFlash_C" _returnvalue_2 "Undefined" 0 0)
                      (Utilities|FlowControl|Delay 0.4)
                      (bind (_outhit _returnvalue_4) (Collision|LineTraceByChannel _returnvalue_3 (+ (* (Math|Vector|GetForwardVector (Transformation|GetWorldRotation _bulletspawn)) 4e+03) _returnvalue_3) "TraceTypeQuery1" false 0 "ForOneFrame"))
                      (if _returnvalue_4
                        (Game|SpawnActorfromClass "/Game/Assets/Weapons/Guns/Explosion.Explosion_C" (Math|Conversions|ToTransform(Vector) (.Location (Collision|BreakHitResult _outhit))) "Undefined" 0 0)
                        (Variables|Default|SetIsFiring false)
                        (goto _label_4 Reset))))))))))
      (elif (>= (- (Utilities|Time|GetGameTimeinSeconds) (Variables|Default|GetTIdleStart)) (Variables|Default|GetIdleDelay)) ; Being lazy?
        ;[1 1 1] RoamState
        (if (not (Variables|Default|GetIsMoving))
          (AI|AIMoveTo self (Class|NavigationSystem|GetRandomPointinNavigableRadius (Transformation|GetWorldLocation (Variables|Character|GetMesh)) 4e+02) 0 2.0 false
            (:then
              (Variables|Default|SetIsMoving true)
              (Variables|Default|SetRoamState true)
              (Variables|Default|SetCombatState false)
              (Variables|Default|SetIdleState false))
            (:OnSuccess
              (Variables|Default|SetIsMoving false :!label _label_8)
              (Variables|Default|SetRoamState false)
              (Variables|Default|SetCombatState false)
              (Variables|Default|SetIdleState true)
              (Variables|Default|SetTIdleStart (Utilities|Time|GetGameTimeinSeconds))
              ;[1 1 1] EnemyIsVisible Check
              (bind _targetisvisible_2 (CallFunction|AIVisionCheck (Variables|Default|GetAIReference) (Variables|Default|GetEnemy) :!label _label_9))
              (Variables|Default|SetEnemyIsVisible _targetisvisible_2))
            (:OnFail
              (goto _label_8))))
        (else
          (goto _label_9))))
    (else
      ;[1 1 1] StateWaterfall
      (if (Variables|Default|GetRoamState) ; Having a look about?
        (Variables|/Script/Engine.CharacterMovementComponent|SetMaxWalkSpeed (Variables|/Script/Engine.Character|GetCharacterMovement (Variables|Default|GetAIReference)) (* (/ (Variables|Default|GetAISpeed) 3.0) 2.0))
        (goto _label_9)
        (elif (Variables|Default|GetCombatState) ; Ya raising hell mate?
          (Variables|/Script/Engine.CharacterMovementComponent|SetMaxWalkSpeed (Variables|/Script/Engine.Character|GetCharacterMovement (Variables|Default|GetAIReference)) (* (/ (Variables|Default|GetAISpeed) 2.5) 3.0))
          (goto _label_3)
          (elif (Variables|Default|GetFleeState) ; Ya fucking off? good
            (Variables|/Script/Engine.CharacterMovementComponent|SetMaxWalkSpeed (Variables|/Script/Engine.Character|GetCharacterMovement (Variables|Default|GetAIReference)) (Variables|Default|GetAISpeed))))))))

(fn ConstructionScript)

(fn AIAim
  (params (TargetActor :type Actor%20Object%20Reference))
  (return (Math|Rotator|FindLookatRotation (Transformation|GetActorLocation (Variables|Default|GetAIReference)) (Transformation|GetActorLocation TargetActor))))

(fn AIVisionCheck
  (params (SearchActor :type Actor%20Object%20Reference) (TargetActor :type Actor%20Object%20Reference))
  (bind _returnvalue (Transformation|GetActorLocation SearchActor))
  (bind _returnvalue_2 (Transformation|GetActorLocation TargetActor))
  (bind _returnvalue_3 (Collision|LineTraceByChannel _returnvalue _returnvalue_2 "TraceTypeQuery1" false 0 "None"))
  (bind _output_get (LocalVariables|SetLineTraceBlocked _returnvalue_3))
  (if _output_get ; Path open
    (LocalVariables|SetTargetVisible false :!label _label)
    (elif (<= (Math|Vector|VectorLength (- _returnvalue_2 _returnvalue)) 5e+03) ; Closer than 150m
      (LocalVariables|SetTargetVisible true)
      (LocalVariables|SetCurrentLocation _returnvalue_2)
      (else
        (goto _label))))
  (return (LocalVariables|GetTargetVisible) (LocalVariables|GetCurrentLocation)))

(fn AIStepTowards
  (params (TargetActor :type Actor%20Object%20Reference))
  (bind _returnvalue (Transformation|GetActorLocation TargetActor))
  (bind _aireference (Variables|Default|GetAIReference))
  (bind _returnvalue_2 (Transformation|GetActorLocation _aireference))
  (return (+ (* (Transformation|GetActorForwardVector _aireference) (/ (Math|Vector|VectorLength (- _returnvalue _returnvalue_2)) 4.0)) _returnvalue_2) _returnvalue))