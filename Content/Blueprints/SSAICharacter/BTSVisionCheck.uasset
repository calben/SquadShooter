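; Behavior Tree service that gives SSAI characters a simple vision check on the player.
; On activation it sets the state key to the first SSAI state and stores the player character as the current enemy.
; Each tick it compares the pawn's forward vector with the direction to the player, switching to the second state inside a 55-degree half-angle.
; The check is angle-only, without distance or line-of-sight tests.
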(event EventReceiveTickAI
  (params (OwnerController :type AI%20Controller%20Object%20Reference) (ControlledPawn :type Pawn%20Object%20Reference) (DeltaSeconds :type Float%20%28single-precision%29))
  (Utilities|FlowControl|Sequence
    (:then_0
      ;[1 1 1] Visibility Check
      (if (< (Class|KismetMathLibrary|DegAcos (Math|Vector|DotProduct (Math|Vector|Normalize (- (Transformation|GetActorLocation (Game|GetPlayerCharacter 0)) (Transformation|GetActorLocation ControlledPawn))) (Transformation|GetActorForwardVector ControlledPawn))) 55.0)
        (Class|BTFunctionLibrary|SetBlackboardValueasEnum (Variables|Default|GetState_VC) (Utilities|Enum|LiteralenumSSAIState "NewEnumerator1"))
        (Class|BTFunctionLibrary|SetBlackboardValueasObject (Variables|Default|GetCurrentEnemy_VC) (Game|GetPlayerCharacter 0))))))

(event EventReceiveActivationAI
  (params (OwnerController :type AI%20Controller%20Object%20Reference) (ControlledPawn :type Pawn%20Object%20Reference))
  (Class|BTFunctionLibrary|SetBlackboardValueasEnum (Variables|Default|GetState_VC) (Utilities|Enum|LiteralenumSSAIState "NewEnumerator0"))
  (Class|BTFunctionLibrary|SetBlackboardValueasObject (Variables|Default|GetCurrentEnemy_VC) (Game|GetPlayerCharacter 0)))