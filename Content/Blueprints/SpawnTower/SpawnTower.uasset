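; SpawnTower is a destructible portal that spawns SSAICharacterC AI characters with a DeathExplosion effect.
; It spawns one AI in front of the portal along Forward, at height SpawnZ, on BeginPlay and on every hit until death.
; DamageActor lowers PortalHealth, calls SpawnAI, and at zero health spawns an explosion at the Heart and destroys the tower.
; A DoOnce gate resets while health remains, so destruction runs once.
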(event EventBeginPlay
  (bind _portal (Variables|Default|GetPortal))
  (bind _forward (Variables|Default|GetForward))
  (bind _returnvalue (Transformation|GetWorldTransform _portal))
  (bind _returnvalue_2 (Math|Vector|GetForwardVector _forward))
  (bind _returnvalue_3 (* _returnvalue_2 5e+02))
  (bind _returnvalue_4 (+ (.location _returnvalue) _returnvalue_3))
  (Game|SpawnActorfromClass "/Game/Assets/Weapons/Guns/DeathExplosion.DeathExplosion_C" (Transformation|GetWorldTransform _portal) "Undefined" 0 0)
  (Game|SpawnActorfromClass "/Game/Blueprints/SSAICharacter/SSAICharacterC.SSAICharacterC_C" (Math|Transform|MakeTransform (Math|Vector|MakeVector (.x _returnvalue_4) (.y _returnvalue_4) (Variables|Default|GetSpawnZ)) (.rotation _returnvalue) "1.000000,1.000000,1.000000") "Undefined" 0 0)
  (Variables|Default|SetAINumber 1)
  (Variables|Default|SetPortalHealth (Variables|Default|GetMaxHealth)))

(event EventDamageActor
  (params (DamageAmount :type Float%20%28single-precision%29))
  (bind _output_get (Variables|Default|SetPortalHealth (- (Variables|Default|GetPortalHealth) DamageAmount)))
  (Utilities|FlowControl|DoOnce false :!label _label
    (:Completed
      (CallFunction|SpawnAI 1)
      (if (<= _output_get 0.0)
        (bind _returnvalue (Game|SpawnActorfromClass "/Game/Assets/Weapons/Guns/DeathExplosion.DeathExplosion_C" (Transformation|GetWorldTransform (Variables|Default|GetHeart)) "Undefined" 0 0))
        (Actor|DestroyActor)
        (Utilities|FlowControl|Delay 3.0)
        (Actor|DestroyActor _returnvalue)
        (else
          (goto _label Reset))))))

(fn ConstructionScript)

(fn SpawnAI
  (params (SpawnNumber :type Integer))
  (bind _portal (Variables|Default|GetPortal))
  (bind _forward (Variables|Default|GetForward))
  (bind _returnvalue (Transformation|GetWorldTransform _portal))
  (bind _returnvalue_2 (Math|Vector|GetForwardVector _forward))
  (bind _returnvalue_3 (* _returnvalue_2 5e+02))
  (bind _returnvalue_4 (+ (.location _returnvalue) _returnvalue_3))
  (Game|SpawnActorfromClass "/Game/Assets/Weapons/Guns/DeathExplosion.DeathExplosion_C" (Transformation|GetWorldTransform _portal) "Undefined" 0 0)
  (Game|SpawnActorfromClass "/Game/Blueprints/SSAICharacter/SSAICharacterC.SSAICharacterC_C" (Math|Transform|MakeTransform (Math|Vector|MakeVector (.x _returnvalue_4) (.y _returnvalue_4) (Variables|Default|GetSpawnZ)) (.rotation _returnvalue) "1.000000,1.000000,1.000000") "Undefined" 0 0))