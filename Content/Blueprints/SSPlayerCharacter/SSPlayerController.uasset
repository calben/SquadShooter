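; SSPlayerController is a player controller Blueprint that tracks the current controlling input device and its sensitivity.
; Getter and setter functions expose the device, while sensitivity is read and written through switches on device type.
; GetSensitivity uses either the current device or a specified one, chosen by a boolean.
; Only the Mouse case is handled, so other devices get the local default on read and no change on write.
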(fn ConstructionScript)

(fn GetControllingDevice
  (return (Variables|Default|GetCurrentControllingDevice)))

(fn SetControllingDevice
  (params (New%20Controlling%20Device :type Byte))
  (Variables|Default|SetCurrentControllingDevice New%20Controlling%20Device))

(fn GetSensitivity
  (params (WhichDevice :type Byte) (CurrentDevice? :type Boolean))
  (Utilities|FlowControl|Sequence
    (:then_0
      (if CurrentDevice?
        (switch Utilities|FlowControl|Switch|Switchon (Variables|Default|GetCurrentControllingDevice)
          (:NewEnumerator0
            (Variables|Default|SetLocalSensitivity (Variables|Default|GetMouseSensitivityCurrent))))
        (else
          (switch Utilities|FlowControl|Switch|Switchon WhichDevice
            (:NewEnumerator0
              (Variables|Default|SetLocalSensitivity (Variables|Default|GetMouseSensitivityCurrent)))))))
    (:then_1
      (return (Variables|Default|GetLocalSensitivity)))))

(fn SetSensitivity
  (params (WhichDevice :type Byte) (NewSensitivity :type Float%20%28single-precision%29))
  (switch Utilities|FlowControl|Switch|Switchon WhichDevice
    (:NewEnumerator0
      (Variables|Default|SetMouseSensitivityCurrent NewSensitivity))))