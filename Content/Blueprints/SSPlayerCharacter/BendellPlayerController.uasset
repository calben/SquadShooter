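; BendellPlayerController tracks the player's current controlling device and stores input sensitivity for it.
; Getter and setter functions expose the active device, and sensitivity reads can target either that device or a specified one.
; Both sensitivity functions switch on the device type, with only the Mouse case handled.
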(fn ConstructionScript)

(fn GetControllingDevice
  (return (Variables|Default|GetCurrentControllingDevice)))

(fn SetControllingDevice
  (params (New%20Controlling%20Device :type BendellControllingDevice%20Enum))
  (Variables|Default|SetCurrentControllingDevice New%20Controlling%20Device))

(fn GetSensitivity
  (params (WhichDevice :type BendellControllingDevice%20Enum) (CurrentDevice? :type Boolean))
  (Utilities|FlowControl|Sequence
    (:then_0
      (if CurrentDevice?
        (switch Utilities|FlowControl|Switch|SwitchonBendellControllingDevice (Variables|Default|GetCurrentControllingDevice)
          (:NewEnumerator0
            (Variables|Default|SetLocalSensitivity (Variables|Default|GetMouseSensitivityCurrent))))
        (else
          (switch Utilities|FlowControl|Switch|SwitchonBendellControllingDevice WhichDevice
            (:NewEnumerator0
              (Variables|Default|SetLocalSensitivity (Variables|Default|GetMouseSensitivityCurrent)))))))
    (:then_1
      (return (Variables|Default|GetLocalSensitivity)))))

(fn SetSensitivity
  (params (WhichDevice :type BendellControllingDevice%20Enum) (NewSensitivity :type Float%20%28single-precision%29))
  (switch Utilities|FlowControl|Switch|SwitchonBendellControllingDevice WhichDevice
    (:NewEnumerator0
      (Variables|Default|SetMouseSensitivityCurrent NewSensitivity))))