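; SpawnOrb is a destructible enemy portal that spawns AI in front of itself, starting with one enemy at BeginPlay.
; Tick compares game time to thresholds set at BeginPlay to fire four one-shot waves of random size, up to five.
; SpawnWave places enemies at fixed offsets via SpawnAI, which randomly picks SSAICharacterC or SSMeleeAI.
; Each hit lowers PortalHealth and spawns two more enemies; at zero the orb explodes and destroys itself.
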(event EventBeginPlay
  (bind _returnvalue (Utilities|Time|GetGameTimeinSeconds))
  (bind _portal (Variables|Default|GetPortal))
  (bind _forward (Variables|Default|GetForward))
  (bind _returnvalue_2 (Transformation|GetWorldTransform _portal))
  (bind _returnvalue_3 (Math|Vector|GetForwardVector _forward))
  (bind _returnvalue_4 (+ _returnvalue 1e+01))
  (bind _returnvalue_5 (* _returnvalue_3 5e+02))
  (bind _returnvalue_6 (+ _returnvalue_4 1e+01))
  (bind _returnvalue_7 (+ (.location _returnvalue_2) _returnvalue_5))
  (bind _returnvalue_8 (+ _returnvalue_6 5.0))
  ;[1 1 1] Set Wave Times, Spawn 1 enemy
  (Utilities|FlowControl|Sequence
    (:then_0
      (Variables|Default|SetT0 _returnvalue)
      (Variables|Default|SetT_Wave1 _returnvalue_4)
      (Variables|Default|SetT_Wave2 _returnvalue_6)
      (Variables|Default|SetT_Wave3 _returnvalue_8)
      (Variables|Default|SetT_Wave4 (+ _returnvalue_8 5.0)))
    (:then_1
      (Game|SpawnActorfromClass "/Game/Blueprints/Equippables/Weapons/WeaponEffects/DeathExplosion.DeathExplosion_C" (Transformation|GetWorldTransform _portal) "Undefined" 0 0)
      (bind _returnvalue_9 (Game|SpawnActorfromClass "/Game/Blueprints/SSAICharacters/RifleAI/SSAICharacterC.SSAICharacterC_C" (Math|Transform|MakeTransform (Math|Vector|MakeVector (.x _returnvalue_7) (.y _returnvalue_7) (Variables|Default|GetSpawnZ)) "0, 0, 0" "1.000000,1.000000,1.000000") "Undefined" 0 0))
      (Variables|Default|SetPortalHealth (Variables|Default|GetMaxHealth))
      (Pawn|SpawnDefaultController _returnvalue_9))))

(event EventTick
  (params (DeltaSeconds :type Float%20%28single-precision%29))
  (bind _returnvalue (Utilities|Time|GetGameTimeinSeconds))
  (bind _returnvalue_2 (Utilities|Time|GetGameTimeinSeconds))
  (bind _returnvalue_3 (Utilities|Time|GetGameTimeinSeconds))
  (bind _returnvalue_4 (Math|Random|RandomIntegerinRange 0 5))
  (bind _returnvalue_5 (Math|Random|RandomIntegerinRange 0 5))
  (bind _returnvalue_6 (Math|Random|RandomIntegerinRange 0 5))
  (bind _returnvalue_7 (Math|Random|RandomIntegerinRange 0 5))
  (bind _t_wave2 (Variables|Default|GetT_Wave2))
  (bind _t_wave3 (Variables|Default|GetT_Wave3))
  (bind _t_wave4 (Variables|Default|GetT_Wave4))
  ;[1 1 1] SpawnWaves
  (if (> (Utilities|Time|GetGameTimeinSeconds) (Variables|Default|GetT_Wave1))
    (if (< _returnvalue_2 _t_wave2)
      (Utilities|FlowControl|DoOnce false
        (:Completed
          (CallFunction|SpawnWave _returnvalue_5)
          (Development|PrintString "wave 1")
          (Development|PrintString (Utilities|String|ToString(Integer) _returnvalue_5))))
      (else
        (if (> _returnvalue_2 _t_wave2) :!label _label
          (if (< _returnvalue_3 _t_wave3)
            (Utilities|FlowControl|DoOnce false
              (:Completed
                (CallFunction|SpawnWave _returnvalue_6)
                (Development|PrintString "wave 2")
                (Development|PrintString (Utilities|String|ToString(Integer) _returnvalue_6))))
            (else
              (if (> _returnvalue_3 _t_wave3) :!label _label_2
                (if (< _returnvalue _t_wave4)
                  (Utilities|FlowControl|DoOnce false
                    (:Completed
                      (CallFunction|SpawnWave _returnvalue_7)
                      (Development|PrintString "Wave 3")
                      (Development|PrintString (Utilities|String|ToString(Integer) _returnvalue_7))))
                  (else
                    (if (> _returnvalue _t_wave4) :!label _label_3
                      (Utilities|FlowControl|DoOnce false
                        (:Completed
                          (CallFunction|SpawnWave _returnvalue_4)
                          (Development|PrintString "wave 4")
                          (Development|PrintString (Utilities|String|ToString(Integer) _returnvalue_4)))))))
                (else
                  (goto _label_3)))))
          (else
            (goto _label_2)))))
    (else
      (goto _label))))

(event EventDamageActor
  (params (DamageAmount :type Float%20%28single-precision%29))
  ;[1 1 1] Spawn 1 when damaged
  (bind _output_get (Variables|Default|SetPortalHealth (- (Variables|Default|GetPortalHealth) DamageAmount)))
  (Utilities|FlowControl|DoOnce false :!label _label
    (:Completed
      (CallFunction|SpawnWave 2)
      (if (<= _output_get 0.0)
        (bind _returnvalue (Game|SpawnActorfromClass "/Game/Blueprints/Equippables/Weapons/WeaponEffects/DeathExplosion.DeathExplosion_C" (Transformation|GetWorldTransform (Variables|Default|GetHeart)) "Undefined" 0 0))
        (Actor|DestroyActor)
        (Utilities|FlowControl|Delay 3.0)
        (Actor|DestroyActor _returnvalue)
        (else
          (goto _label Reset))))))

(fn ConstructionScript)

(fn SpawnAI
  (params (SpawnTransform :type Transform))
  (Game|SpawnActorfromClass "/Game/Blueprints/Equippables/Weapons/WeaponEffects/DeathExplosion.DeathExplosion_C" (Transformation|GetWorldTransform (Variables|Default|GetPortal)) "Undefined" 0 0)
  (if (>= (Math|Random|RandomIntegerinRange 0 10) 5)
    (bind _returnvalue (Game|SpawnActorfromClass "/Game/Blueprints/SSAICharacters/RifleAI/SSAICharacterC.SSAICharacterC_C" SpawnTransform "Undefined" 0 0))
    (Pawn|SpawnDefaultController _returnvalue)
    (else
      (bind _returnvalue_2 (Game|SpawnActorfromClass "/Game/Blueprints/SSAICharacters/MeleeAI/SSMeleeAI.SSMeleeAI_C" SpawnTransform "Undefined" 0 0))
      (Pawn|SpawnDefaultController _returnvalue_2))))

(fn SpawnWave
  (params (EnemyCount :type Integer))
  (bind _portal (Variables|Default|GetPortal))
  (bind _spawnz (Variables|Default|GetSpawnZ))
  (bind _forward (Variables|Default|GetForward))
  (bind _spawnz_2 (Variables|Default|GetSpawnZ))
  (bind _spawnz_3 (Variables|Default|GetSpawnZ))
  (bind _spawnz_4 (Variables|Default|GetSpawnZ))
  (bind _returnvalue (Transformation|GetWorldTransform _portal))
  (bind _returnvalue_2 (Math|Vector|GetForwardVector _forward))
  (bind _returnvalue_3 (* _returnvalue_2 5e+02))
  (bind _returnvalue_4 (+ (.location _returnvalue) _returnvalue_3))
  (bind _returnvalue_5 (Math|Transform|MakeTransform (Math|Vector|MakeVector (.x _returnvalue_4) (.y _returnvalue_4) _spawnz) "0, 0, 0" "1.000000,1.000000,1.000000"))
  (bind _returnvalue_6 (+ (.y _returnvalue_4) -2e+02))
  (bind _returnvalue_7 (+ (.x _returnvalue_4) -1e+02))
  (bind _returnvalue_8 (+ (.x _returnvalue_4) -1e+02))
  (bind _returnvalue_9 (+ (.y _returnvalue_4) 2e+02))
  (bind _returnvalue_10 (Math|Transform|MakeTransform (Math|Vector|MakeVector _returnvalue_8 _returnvalue_9 _spawnz_4) "0, 0, 0" "1.000000,1.000000,1.000000"))
  (bind _returnvalue_11 (Math|Transform|MakeTransform (Math|Vector|MakeVector _returnvalue_7 _returnvalue_6 _spawnz_3) "0, 0, 0" "1.000000,1.000000,1.000000"))
  (bind _returnvalue_12 (+ _returnvalue_8 -1e+02))
  (bind _returnvalue_13 (+ _returnvalue_9 2e+02))
  (bind _returnvalue_14 (Math|Transform|MakeTransform (Math|Vector|MakeVector _returnvalue_12 _returnvalue_13 _spawnz_2) "0, 0, 0" "1.000000,1.000000,1.000000"))
  (if (not (== EnemyCount 0))
    (if (== EnemyCount 1)
      (CallFunction|SpawnAI _returnvalue_5)
      (elif (== EnemyCount 2)
        (CallFunction|SpawnAI _returnvalue_5)
        (CallFunction|SpawnAI _returnvalue_10)
        (elif (== EnemyCount 3)
          (CallFunction|SpawnAI _returnvalue_5)
          (CallFunction|SpawnAI _returnvalue_10)
          (CallFunction|SpawnAI _returnvalue_11)
          (elif (== EnemyCount 4)
            (CallFunction|SpawnAI _returnvalue_5)
            (CallFunction|SpawnAI _returnvalue_10)
            (CallFunction|SpawnAI _returnvalue_11)
            (CallFunction|SpawnAI _returnvalue_14)
            (elif (== EnemyCount 5)
              (CallFunction|SpawnAI _returnvalue_5)
              (CallFunction|SpawnAI _returnvalue_10)
              (CallFunction|SpawnAI _returnvalue_11)
              (CallFunction|SpawnAI _returnvalue_14)
              (CallFunction|SpawnAI (Math|Transform|MakeTransform (Math|Vector|MakeVector (+ _returnvalue_7 -1e+02) (+ _returnvalue_6 -2e+02) (Variables|Default|GetSpawnZ)) "0, 0, 0" "1.000000,1.000000,1.000000")))))))))